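; BP_TCP is a TCP client Blueprint that turns messages from a local server, apparently gesture data, into a Grab flag.
; It calls Connect on every Tick, and on connection starts a looping timer for "Recieve gesture data", a function absent from this file.
; Incoming strings set Grab true for "잡기" (grab) and false otherwise, printing the result.
; EndPlay disconnects connection 0.
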(event Custom|Disconnected
  (params (ConnectionId :type Integer)))

(event Custom|Connected
  (params (ConnectionId :type Integer))
  (if true
    (Development|PrintString "connected")
    (Utilities|Time|SetTimerbyFunctionName 0 "Recieve gesture data" 0.1 true)))

(event Custom|Message
  (params (ConnectionId :type Integer) (Message :type Array%20of%20Bytes))
  (bind _returnvalue (Class|TcpSocketConnection|MessageReadString Message (Utilities|Array|Length Message)))
  (if (Utilities|Enum|Equal(Enum) _returnvalue "잡기")
    (Development|PrintString "잡았다")
    (Variables|Default|SetbGrab true)
    (else
      (Development|PrintString "놓기")
      (Variables|Default|SetbGrab false))))

(event Collision|EventActorBeginOverlap
  (params (OtherActor :type Actor%20Object%20Reference)))

(event EventEndPlay
  (params (EndPlayReason :type EEndPlayReason%20Enum :default "Destroyed"))
  (Class|TcpSocketConnection|Disconnect))

(event EventTick
  (params (DeltaSeconds :type Float%20%28single-precision%29))
  (Class|TcpSocketConnection|Connect "127.0.0.1" 65432 (delegate Custom|Disconnected) (delegate Custom|Connected) (delegate Custom|Message)))

(fn ConstructionScript)