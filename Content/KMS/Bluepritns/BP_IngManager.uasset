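; Ingredient manager that gathers the level's food ingredient actors, such as banana, beef and noodle, into a single array.
; On BeginPlay, a Sequence looks up one actor per ingredient Blueprint class with GetActorOfClass.
; Every branch then re-sets IngArr from all fourteen lookup results, so the array is only fully populated after the last one.
; The file contains no other logic and does not itself use the array.
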(event EventBeginPlay
  ;[1 1 1] 재료들 배열에 넣기
  (Utilities|FlowControl|Sequence
    (:then_0
      (bind _returnvalue (Actor|GetActorOfClass "/Game/KMS/Bluepritns/Ingredients/BP_Banana.BP_Banana_C")))
    (:then_1
      (bind _returnvalue_2 (Actor|GetActorOfClass "/Game/KMS/Bluepritns/Ingredients/BP_Brocoli.BP_Brocoli_C")))
    (:then_2
      (bind _returnvalue_3 (Actor|GetActorOfClass "/Game/KMS/Bluepritns/Ingredients/BP_Beef.BP_Beef_C")))
    (:then_3
      (bind _returnvalue_4 (Actor|GetActorOfClass "/Game/KMS/Bluepritns/Ingredients/BP_Noodle.BP_Noodle_C")))
    (:then_4
      (bind _returnvalue_5 (Actor|GetActorOfClass "/Game/KMS/Bluepritns/Ingredients/BP_ChilPepper.BP_ChilPepper_C")))
    (:then_5
      (bind _returnvalue_6 (Actor|GetActorOfClass "/Game/KMS/Bluepritns/Ingredients/BP_Soup.BP_Soup_C")))
    (:then_6
      (bind _returnvalue_7 (Actor|GetActorOfClass "/Game/KMS/Bluepritns/Ingredients/BP_Egg.BP_Egg_C")))
    (:then_7
      (bind _returnvalue_8 (Actor|GetActorOfClass "/Game/KMS/Bluepritns/Ingredients/BP_Mushroom.BP_Mushroom_C")))
    (:then_8
      (bind _returnvalue_9 (Actor|GetActorOfClass "/Game/KMS/Bluepritns/Ingredients/BP_Garlic.BP_Garlic_C")))
    (:then_9
      (bind _returnvalue_10 (Actor|GetActorOfClass "/Game/KMS/Bluepritns/Ingredients/BP_Strawberry.BP_Strawberry_C")))
    (:then_10
      (bind _returnvalue_11 (Actor|GetActorOfClass "/Game/KMS/Bluepritns/Ingredients/BP_Carrot.BP_Carrot_C")))
    (:then_11
      (bind _returnvalue_12 (Actor|GetActorOfClass "/Game/KMS/Bluepritns/Ingredients/BP_SpringOnion.BP_SpringOnion_C")))
    (:then_12
      (bind _returnvalue_13 (Actor|GetActorOfClass "/Game/KMS/Bluepritns/Ingredients/BP_Potato.BP_Potato_C")))
    (:then_13
      (bind _returnvalue_14 (Actor|GetActorOfClass "/Game/KMS/Bluepritns/Ingredients/BP_Pumkin.BP_Pumkin_C"))))
  (Variables|Default|SetIngArr (Utilities|Array|MakeArray _returnvalue _returnvalue_2 _returnvalue_3 _returnvalue_4 _returnvalue_5 _returnvalue_6 _returnvalue_7 _returnvalue_8 _returnvalue_9 _returnvalue_10 _returnvalue_11 _returnvalue_12 _returnvalue_13 _returnvalue_14)))

(event Collision|EventActorBeginOverlap
  (params (OtherActor :type Actor%20Object%20Reference)))

(event EventTick
  (params (DeltaSeconds :type Float%20%28single-precision%29)))

(fn ConstructionScript)