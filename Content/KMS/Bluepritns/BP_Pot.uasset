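; BP_Pot is a pot actor that checks overlapping actors against food ingredient Blueprints.
; On ActorBeginOverlap, a Sequence runs a separate cast of the other actor for each ingredient type, from produce to beef, egg, noodle and soup.
; No logic follows any cast, so overlaps currently have no effect.
; BeginPlay, Tick and the construction script are empty.
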(event EventBeginPlay)

(event Collision|EventActorBeginOverlap
  (params (OtherActor :type Actor%20Object%20Reference))
  (Utilities|FlowControl|Sequence
    (:then_0
      (Utilities|Casting|CastToBP_Banana OtherActor))
    (:then_1
      (Utilities|Casting|CastToBP_SpringOnion OtherActor))
    (:then_2
      (Utilities|Casting|CastToBP_Soup OtherActor))
    (:then_3
      (Utilities|Casting|CastToBP_Noodle OtherActor))
    (:then_4
      (Utilities|Casting|CastToBP_Mushroom OtherActor))
    (:then_5
      (Utilities|Casting|CastToBP_Beef OtherActor))
    (:then_6
      (Utilities|Casting|CastToBP_Mango OtherActor))
    (:then_7
      (Utilities|Casting|CastToBP_Strawberry OtherActor))
    (:then_8
      (Utilities|Casting|CastToBP_Egg OtherActor))
    (:then_9
      (Utilities|Casting|CastToBP_Potato OtherActor))
    (:then_10
      (Utilities|Casting|CastToBP_Brocoli OtherActor))
    (:then_11
      (Utilities|Casting|CastToBP_Carrot OtherActor))
    (:then_12
      (Utilities|Casting|CastToBP_Garlic OtherActor))
    (:then_13
      (Utilities|Casting|CastToBP_Pumkin OtherActor))
    (:then_14
      (Utilities|Casting|CastToBP_ChilPepper OtherActor))
    (:then_15
      (Utilities|Casting|CastToBP_BeanSprout OtherActor))))

(event EventTick
  (params (DeltaSeconds :type Float%20%28single-precision%29)))

(fn ConstructionScript)